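; Game mode for a timed drinking-and-smoking challenge, won by finishing four beers and two cigarettes.
; Interface-style events start the timer and count each finished beer or cigarette, while Tick accumulates elapsed time as the timer runs.
; Each count update calls CheckWinCondition, which stops the timer, flags completion and reports the final time through Print String once both targets are met.
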(event `self.ReceiveTick`
  (params (DeltaSeconds :type "Float (single-precision)"))
  (if (`self.TimerRunning`)
    (bind _output_get (set `self.ElapsedTime` (+ (`self.ElapsedTime`) DeltaSeconds)))))

(event `/Game/Tektonika25/PetersonsHugo/BPI_GameEvents.BeerFinishedBPI`
  (bind _output_get (set `self.BeersConsumed` (+ (`self.BeersConsumed`) 1)))
  (`self.CheckWinCondition`)
  (`KismetSystemLibrary.PrintString` (`KismetStringLibrary.Conv_IntToString` _output_get)))

(event `/Game/Tektonika25/PetersonsHugo/BPI_GameEvents.CigFinishedBPI`
  (bind _output_get (set `self.CigsSmoked` (+ (`self.CigsSmoked`) 1)))
  (`self.CheckWinCondition`)
  (`KismetSystemLibrary.PrintString` (`KismetStringLibrary.Conv_IntToString` _output_get)))

(event `/Game/Tektonika25/PetersonsHugo/BPI_GameEvents.StartTimerBPI`
  (set `self.TimerRunning` true)
  (`KismetSystemLibrary.PrintString` "Challenge Started"))

(fn `CheckWinCondition`
  (if (and (>= (`self.BeersConsumed`) 4) (>= (`self.CigsSmoked`) 2))
    (set `self.TimerRunning` false)
    (set `self.ChallengeComplete` true)
    (`KismetSystemLibrary.PrintString` (`KismetStringLibrary.BuildString_Double` "Challenge complete! Time: " "sec" (`self.ElapsedTime`)))))

(fn `UserConstructionScript`)