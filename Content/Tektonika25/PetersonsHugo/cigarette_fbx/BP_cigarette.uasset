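; Cigarette actor that burns down while something overlaps its SmokeZone and reports to the game mode when finished.
; Overlap begin lights it and starts a delayed loop that reduces the length and prints it; overlap end stops it.
; Tick applies the length to the model's X scale while smoking.
; Once the length bottoms out, a one-time interface message tells the game mode.
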(event `self.ReceiveTick`
  (params (DeltaSeconds :type "Float (single-precision)"))
  (if (== (`self.IsLit`) true)
    (if (== (`self.CanSmoke`) true)
      (`SceneComponent.SetRelativeScale3D` (`self.Cig_model`) (`KismetMathLibrary.MakeVector` (stale `self.SmokeZone.OnComponentBeginOverlap` _output_get) 1.0 1.0)))))

(event `self.SmokeZone.OnComponentBeginOverlap`
  (params (OverlappedComponent :type "PrimitiveComponent Object Reference") (OtherActor :type "Actor Object Reference") (OtherComp :type "PrimitiveComponent Object Reference") (OtherBodyIndex :type Integer) (bFromSweep :type Boolean) (SweepResult :type "HitResult Structure (by ref)"))
  (set `self.IsLit` true)
  (if (`self.IsLit`) :!label _label
    (if (> (`self.CigaretteLenght`) 0.04)
      (set `self.CanSmoke` true)
      (`KismetSystemLibrary.Delay` 0.2)
      (bind _output_get (set `self.CigaretteLenght` (- (`self.CigaretteLenght`) 0.05)))
      (`KismetSystemLibrary.PrintString` (`KismetStringLibrary.Conv_DoubleToString` _output_get))
      (goto _label)
      (elif (== (`self.HasBeenCounted`) false)
        (message `/Game/Tektonika25/PetersonsHugo/BPI_GameEvents.CigFinishedBPI` (`GameplayStatics.GetGameMode`))
        (set `self.HasBeenCounted` true)))))

(event `self.SmokeZone.OnComponentEndOverlap`
  (params (OverlappedComponent :type "PrimitiveComponent Object Reference") (OtherActor :type "Actor Object Reference") (OtherComp :type "PrimitiveComponent Object Reference") (OtherBodyIndex :type Integer))
  (set `self.IsLit` false)
  (set `self.CanSmoke` false)
  (set `self.CigaretteLenght` (`self.CigaretteLenght`)))

(fn `UserConstructionScript`)