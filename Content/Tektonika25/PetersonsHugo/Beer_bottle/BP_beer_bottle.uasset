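; Beer bottle actor that drains its liquid while something overlaps its DrinkZone component.
; A looping Delay on begin overlap sets CanDrink and lowers LiquidAmount in small steps, printing each new value, until the bottle is nearly empty or the overlap ends.
; When empty, it sends a BeerFinished interface message to the game mode, guarded by HasBeenCounted so it only counts once.
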(event `self.DrinkZone.OnComponentBeginOverlap`
  (params (OverlappedComponent :type "PrimitiveComponent Object Reference") (OtherActor :type "Actor Object Reference") (OtherComp :type "PrimitiveComponent Object Reference") (OtherBodyIndex :type Integer) (bFromSweep :type Boolean) (SweepResult :type "HitResult Structure (by ref)"))
  (set `self.isOverlaping` true)
  (if (`self.isOverlaping`) :!label _label
    (if (> (`self.LiquidAmount`) 0.04)
      (set `self.bCanDrink` true)
      (`KismetSystemLibrary.Delay` 0.2)
      (bind _output_get (set `self.LiquidAmount` (- (`self.LiquidAmount`) 0.05)))
      (`KismetSystemLibrary.PrintString` (`KismetStringLibrary.Conv_DoubleToString` _output_get))
      (goto _label)
      (elif (== (`self.HasBeenCounted`) false)
        (message `/Game/Tektonika25/PetersonsHugo/BPI_GameEvents.BeerFinishedBPI` (`GameplayStatics.GetGameMode`))
        (set `self.HasBeenCounted` true)))))

(event `self.DrinkZone.OnComponentEndOverlap`
  (params (OverlappedComponent :type "PrimitiveComponent Object Reference") (OtherActor :type "Actor Object Reference") (OtherComp :type "PrimitiveComponent Object Reference") (OtherBodyIndex :type Integer))
  (set `self.isOverlaping` false)
  (set `self.bCanDrink` false)
  (set `self.LiquidAmount` (`self.LiquidAmount`)))

(fn `UserConstructionScript`)