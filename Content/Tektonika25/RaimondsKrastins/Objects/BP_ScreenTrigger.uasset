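; BP_ScreenTrigger is a trigger volume that changes the look of a target screen mesh when something overlaps it.
; On CollisionBox overlap, it prints the actor's name and applies a random PossibleMaterials entry, using a fixed index range, to the TargetScreen static mesh actor.
; Disconnected leftover nodes sketch a BP_AnimatedBox filter, a repeat-material check and media player video playback, so any overlapping actor triggers the swap.
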(event `self.ReceiveBeginPlay`)

(event `self.ReceiveActorBeginOverlap`
  (params (OtherActor :type "Actor Object Reference")))

(event `self.CollisionBox.OnComponentBeginOverlap`
  (params (OverlappedComponent :type "PrimitiveComponent Object Reference") (OtherActor :type "Actor Object Reference") (OtherComp :type "PrimitiveComponent Object Reference") (OtherBodyIndex :type Integer) (bFromSweep :type Boolean) (SweepResult :type "HitResult Structure (by ref)"))
  (`KismetSystemLibrary.PrintString` (`KismetSystemLibrary.GetDisplayName` OtherActor))
  (bind _asstatic_mesh_actor (cast `StaticMeshActor` (`self.TargetScreen`)))
  (`PrimitiveComponent.SetMaterial` (`StaticMeshActor.StaticMeshComponent` _asstatic_mesh_actor) 0 (`|GetArrayItem` (`self.PossibleMaterials`) (`KismetMathLibrary.RandomIntegerInRange` 0 5))))

(fn `UserConstructionScript`)