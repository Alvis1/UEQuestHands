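; BP_ScreenTrigger is a trigger actor that changes the look of a target screen when anything overlaps its collision box.
; The overlap applies a random pick from the first six possible materials to the TargetScreen mesh.
; Separately, Tick draws a debug arrow to the Pawn and moves a referenced StaticMeshActor with velocity proportional to that offset, with zero acceleration.
; Video playback and speed-check experiments remain disconnected.
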(event `self.ReceiveBeginPlay`)

(event `self.ReceiveActorBeginOverlap`
  (params (OtherActor :type "Actor Object Reference")))

(event `self.ReceiveHit`
  (params (MyComp :type "PrimitiveComponent Object Reference") (Other :type "Actor Object Reference") (OtherComp :type "PrimitiveComponent Object Reference") (bSelfMoved :type Boolean) (HitLocation :type "Vector Structure") (HitNormal :type "Vector Structure") (NormalImpulse :type "Vector Structure") (Hit :type "HitResult Structure (by ref)")))

(event `self.CollisionBox.OnComponentBeginOverlap`
  (params (OverlappedComponent :type "PrimitiveComponent Object Reference") (OtherActor :type "Actor Object Reference") (OtherComp :type "PrimitiveComponent Object Reference") (OtherBodyIndex :type Integer) (bFromSweep :type Boolean) (SweepResult :type "HitResult Structure (by ref)"))
  (bind _asstatic_mesh_actor (cast `StaticMeshActor` (`self.TargetScreen`)))
  (`PrimitiveComponent.SetMaterial` (`StaticMeshActor.StaticMeshComponent` _asstatic_mesh_actor) 0 (`|GetArrayItem` (`self.PossibleMaterials`) (`KismetMathLibrary.RandomIntegerInRange` 0 5))))

(event `self.CollisionBox.OnComponentHit`
  (params (HitComponent :type "PrimitiveComponent Object Reference") (OtherActor :type "Actor Object Reference") (OtherComp :type "PrimitiveComponent Object Reference") (NormalImpulse :type "Vector Structure") (Hit :type "HitResult Structure (by ref)")))

(event `self.Cube.OnComponentHit`
  (params (HitComponent :type "PrimitiveComponent Object Reference") (OtherActor :type "Actor Object Reference") (OtherComp :type "PrimitiveComponent Object Reference") (NormalImpulse :type "Vector Structure") (Hit :type "HitResult Structure (by ref)")))

(event `self.ReceiveTick`
  (params (DeltaSeconds :type "Float (single-precision)"))
  (bind _staticmeshactor (`self.StaticMeshActor`))
  (bind _returnvalue (`self.K2_GetActorLocation` (`self.Pawn`)))
  (bind _returnvalue_2 (`self.K2_GetActorLocation` self))
  (bind (_returnvalue_x _returnvalue_y _returnvalue_z) (`KismetMathLibrary.BreakVector` (* (- _returnvalue _returnvalue_2) 0.4)))
  ;[1 1 1] Velocity and Acceleration
  (`KismetSystemLibrary.DrawDebugArrow` _returnvalue_2 _returnvalue)
  (bind _output_get (set `self.Velocity` (`KismetMathLibrary.MakeVector` _returnvalue_x _returnvalue_y _returnvalue_z)))
  (set `self.Velocity` (+ (`self.Velocity`) (* (0.0 0.0 0.0) DeltaSeconds)))
  (`self.K2_SetActorLocation` _staticmeshactor (+ (`self.K2_GetActorLocation` _staticmeshactor) (* _output_get DeltaSeconds)) false false))

(fn `UserConstructionScript`)